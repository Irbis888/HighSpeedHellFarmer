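; BP_FireMode_Single is an upgrade fire mode that makes each shot spawn a single entity from the player's first-person camera.
; On Shoot, it builds a transform from the camera's "Ammo" socket location plus a camera-rotated ProjectileOffset, facing along the camera's rotation.
; It passes that transform and its Plant value to the owner component's SpawnEntityAtTransform, which handles the spawning.
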(event EventShoot
  (bind _ownercomponent (Variables|Default|GetOwnerComponent))
  (bind _ownerclass (Variables|/Game/FirstPerson/Blueprints/BP_Leika_Comp.BP_Leika_Comp_C|GetOwnerClass _ownercomponent))
  (bind _firstpersoncamera (Variables|/Game/FarmerChar/BP_FPC_FastRunnerFarmer.BP_FPC_FastRunnerFarmer_C|GetFirstPersonCamera _ownerclass))
  (bind _returnvalue (Transformation|GetWorldRotation _firstpersoncamera))
  (Default|SpawnEntityatTransform (Variables|Default|GetOwnerComponent) (Variables|Default|GetPlant) (Math|Transform|MakeTransform (+ (Transformation|GetSocketLocation _firstpersoncamera "Ammo") (Math|Vector|RotateVector (Variables|Default|GetProjectile%20Offset) _returnvalue)) _returnvalue) "NewEnumerator0"))