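; BP_SeedBomb is a seed bomb actor that bursts into a batch of seed actors.
; It explodes on a short timer started at BeginPlay, or when its sphere begins overlapping BP_Farmland.
; The explosion spawns a configurable number of BP_Seed_P actors at its location, each with random yaw and the bomb's Seed as its plant, then destroys the bomb.
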(event OnComponentBeginOverlap(Sphere1)
  (params (OverlappedComponent :type Primitive%20Component%20Object%20Reference) (OtherActor :type Actor%20Object%20Reference) (OtherComp :type Primitive%20Component%20Object%20Reference) (OtherBodyIndex :type Integer) (bFromSweep :type Boolean) (SweepResult :type Hit%20Result%20Structure%20%28by%20ref%29))
  (Utilities|Casting|CastToBP_Farmland OtherActor)
  (CallFunction|Explode))

(event Custom|Explode
  (for _index (range 1 (Variables|Default|GetAnount))
    (Game|SpawnActorfromClass "/Game/FirstPerson/Blueprints/BP_Seed_P.BP_Seed_P_C" (Math|Transform|MakeTransform (Transformation|GetActorLocation) (Math|Vector|RotatorfromAxisandAngle "0.000000,0.000000,1.000000" (Math|Random|RandomFloatinRange 0.0 3.6e+02))) "Undefined" "MultiplyWithRoot" 0 (Variables|Default|GetSeed) 0))
  (Actor|DestroyActor))

(event EventBeginPlay
  (Utilities|Time|SetTimerbyEvent (delegate Custom|Explode) 2.0))

(fn ConstructionScript)