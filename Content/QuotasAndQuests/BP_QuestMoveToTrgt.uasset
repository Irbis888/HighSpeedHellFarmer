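; Quest objective actor for a "move to target" goal, completed when the first-person character reaches its trigger box.
; Entering the box calls UpdateQuests on the QuestHolder instead of completing the quest directly.
; CheckWin looks for the character among the box's overlapping actors, then latches IsCompleted and prints a Russian debug message.
; Once set, IsCompleted is returned without rechecking, and BeginPlay resets it to false.
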(event OnComponentBeginOverlap(Box)
  (params (OverlappedComponent :type Primitive%20Component%20Object%20Reference) (OtherActor :type Actor%20Object%20Reference) (OtherComp :type Primitive%20Component%20Object%20Reference) (OtherBodyIndex :type Integer) (bFromSweep :type Boolean) (SweepResult :type Hit%20Result%20Structure%20%28by%20ref%29))
  (Utilities|Casting|CastToBP_FirstPersonCharacter OtherActor)
  (Default|UpdateQuests (Variables|Default|GetQuestHolder)))

(event EventBeginPlay
  (|CallParentFunction)
  (Variables|Default|SetIsCompleted false))

(event Collision|EventActorBeginOverlap
  (params (OtherActor :type Actor%20Object%20Reference))
  (|CallParentFunction OtherActor))

(event EventTick
  (params (DeltaSeconds :type Float%20%28single-precision%29))
  (|CallParentFunction DeltaSeconds) ; This node is disabled and will not be called.\nDrag off pins to build functionality.
)

(fn ConstructionScript
  (|CallParentFunction))

(fn CheckWin
  (if (Variables|Default|GetIsCompleted)
    (return (Variables|Default|GetIsCompleted))
    (else
      (for _array_element (Collision|GetOverlappingActors (Variables|Default|GetBox) "/Game/FirstPerson/Blueprints/BP_FirstPersonCharacter.BP_FirstPersonCharacter_C" :!class /Script/Engine.PrimitiveComponent)
        (if (Utilities|IsValid _array_element)
          (Development|PrintString "Вы дошли ддо триггера квеста" true true "(R=0.000000,G=1.000000,B=0.129164,A=1.000000)")
          (Variables|Default|SetIsCompleted true)
          (return true))))))