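; Quest manager actor that runs timed plant-gathering quests, showing the current goal and countdown in a quest widget.
; UpdateQuests checks the current quest's win condition, advancing through QuestList with a sound and wrapping to the first, and resets the timer.
; A Delay on Tick makes the one-second countdown.
; On timeout it fails the quest, shows an end screen with the player's total plants, then opens MainMenu.
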(event EventBeginPlay
  (bind _returnvalue (Game|GetPlayerController 0))
  (bind _output_get (Variables|Default|SetCurentQuestID 0))
  (Variables|Default|SetCurrentQuest (Utilities|Array|Get(acopy) (Variables|Default|GetQuestList) _output_get))
  (bind _returnvalue_2 (UserInterface|CreateWidget "/Game/QuotasAndQuests/WBP_Quest.WBP_Quest_C" _returnvalue))
  (Variables|Default|SetQuestUI _returnvalue_2)
  (bind _returnvalue_3 (UserInterface|CreateWidget "/Game/QuotasAndQuests/WBP_EndScrean.WBP_EndScrean_C" _returnvalue))
  (Variables|Default|SetWBP%20EndScrean _returnvalue_3)
  (CallFunction|UpdateQuests)
  (UserInterface|Viewport|AddtoViewport (Variables|Default|GetQuestUI) 0)
  (CallFunction|SetTimerSeconds))

(event Collision|EventActorBeginOverlap
  (params (OtherActor :type Actor%20Object%20Reference)))

(event EventTick
  (params (DeltaSeconds :type Float%20%28single-precision%29))
  (bind _wbp_endscrean (Variables|Default|GetWBP%20EndScrean))
  (Utilities|FlowControl|Delay 1.0)
  (if (> (Variables|Default|GetTimerSeconds) 0)
    (bind _output_get (Variables|Default|SetTimerSeconds (- (Variables|Default|GetTimerSeconds) 1)))
    (CallFunction|UpdateTimerText _output_get)
    (else
      (Default|FailedQuest (Variables|Default|GetCurrentQuest))
      (Utilities|FlowControl|Delay 2.0)
      (bind _asbp_quest_plant (Utilities|Casting|CastToBP_QuestPlant (Variables|Default|GetCurrentQuest)))
      (Variables|/Script/UMG.TextBlock|SetText (Variables|/Game/QuotasAndQuests/WBP_EndScrean.WBP_EndScrean_C|GetCountTExt _wbp_endscrean) (Utilities|Text|ToText(Integer) (Variables|/Game/FarmerChar/BP_FPC_FastRunnerFarmer.BP_FPC_FastRunnerFarmer_C|GetTotalPlants (.AsBP%20FPC%20Fast%20Runner%20Farmer (Utilities|Casting|CastToBP_FPC_FastRunnerFarmer (Game|GetPlayerCharacter 0))))))
      (UserInterface|Viewport|AddtoViewport _wbp_endscrean 0)
      (Utilities|FlowControl|Delay 4.0)
      (Game|OpenLevel(byName) "MainMenu"))))

(fn ConstructionScript)

(fn GiveNextQuest
  (Math|Integer|IncrementInt (Variables|Default|GetCurentQuestID)
    (:%20%20
      (if (>= (Variables|Default|GetCurentQuestID) (Utilities|Array|Length (Variables|Default|GetQuestList)))
        (Variables|Default|SetCurentQuestID 0))
      (Variables|Default|SetCurrentQuest (Utilities|Array|Get(acopy) (Variables|Default|GetQuestList) (Variables|Default|GetCurentQuestID)))
      (CallFunction|UpdateQuests)
      (Audio|PlaySound2D "/Engine/EditorSounds/Notifications/CompileSuccess_Cue.CompileSuccess_Cue" 1.0 1.0 0.0 0 0))))

(fn UpdateQuests
  (bind _iscompleted (Default|CheckWin (Variables|Default|GetCurrentQuest)))
  (if _iscompleted
    (CallFunction|GiveNextQuest)
    (else
      (Variables|/Script/UMG.TextBlock|SetText (Variables|/Game/QuotasAndQuests/WBP_Quest.WBP_Quest_C|GetHeaderText (Variables|Default|GetQuestUI)) (Utilities|Text|ToText(String) (Utilities|String|Append (Utilities|String|Append "Gather " (Variables|/Game/QuotasAndQuests/BP_Quest.BP_Quest_C|GetHeaderText (Variables|Default|GetCurrentQuest))) " plants")))
      (Variables|/Game/QuotasAndQuests/BP_Quest.BP_Quest_C|SetIsFailed (Variables|Default|GetCurrentQuest) false)))
  (CallFunction|SetTimerSeconds))

(fn SetQuest
  (params (Quest :type BP%20Quest%20Object%20Reference))
  (LocalVariables|SetLocQuest Quest)
  (for (_array_element _array_index) (Variables|Default|GetQuestList)
    (if (== _array_element (LocalVariables|GetLocQuest))
      (Variables|Default|SetCurentQuestID _array_index)
      (Variables|Default|SetCurrentQuest (LocalVariables|GetLocQuest))
      (CallFunction|UpdateQuests))))

(fn UpdateTimerText
  (params (NowTime :type Integer))
  (Variables|/Script/UMG.TextBlock|SetText (Variables|/Game/QuotasAndQuests/WBP_Quest.WBP_Quest_C|GetTimerText (Variables|Default|GetQuestUI)) (Utilities|Text|ToText(Integer) NowTime)))

(fn SetTimerSeconds
  (bind _currentquest (Variables|Default|GetCurrentQuest))
  (bind _completetime (Variables|/Game/QuotasAndQuests/BP_Quest.BP_Quest_C|GetCompleteTime _currentquest))
  (Variables|Default|SetTimerSeconds _completetime)
  (Variables|/Script/UMG.TextBlock|SetText (Variables|/Game/QuotasAndQuests/WBP_Quest.WBP_Quest_C|GetTimerText (Variables|Default|GetQuestUI)) (Utilities|Text|ToText(Integer) _completetime)))