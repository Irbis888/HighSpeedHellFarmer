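; Plant-gathering quest that tracks how many plants the FastRunnerFarmer player has gathered against a growing quota.
; Binds to the player's plant-count update at BeginPlay, then copies the count and tells QuestHolder to update quests.
; CheckConditions extends the parent check: on a met quota it zeroes the player's count, raises the target by a fixed step and refreshes HeaderText.
; Its return compares the stored count to the already-raised target.
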(event Custom|UpdatePlants
  (Variables|Default|SetCurrentPlants (Variables|/Game/FarmerChar/BP_FPC_FastRunnerFarmer.BP_FPC_FastRunnerFarmer_C|GetPlantsGathered (stale EventBeginPlay _output_get)))
  (Development|PrintString "BBBEEEBRA")
  (Default|UpdateQuests (Variables|Default|GetQuestHolder)))

(event EventBeginPlay
  (|CallParentFunction)
  (bind _asbp_fpc_fast_runner_farmer (Utilities|Casting|CastToBP_FPC_FastRunnerFarmer (Game|GetPlayerCharacter 0)))
  (bind _output_get (Variables|Default|SetAsBP_FPC _asbp_fpc_fast_runner_farmer))
  (EventDispatchers|BindEventtoUpdatePlantsCount _output_get (delegate Custom|UpdatePlants)))

(event Collision|EventActorBeginOverlap
  (params (OtherActor :type Actor%20Object%20Reference))
  (|CallParentFunction OtherActor) ; This node is disabled and will not be called.\nDrag off pins to build functionality.
)

(event EventTick
  (params (DeltaSeconds :type Float%20%28single-precision%29))
  (|CallParentFunction DeltaSeconds) ; This node is disabled and will not be called.\nDrag off pins to build functionality.
)

(fn ConstructionScript
  (|CallParentFunction))

(fn CheckConditions
  (|CallParentFunction)
  (if (>= (Variables|Default|GetCurrentPlants) (Variables|Default|GetNeedPlants))
    (bind _returnvalue (Actor|GetActorOfClass "/Game/FarmerChar/BP_FPC_FastRunnerFarmer.BP_FPC_FastRunnerFarmer_C"))
    (bind _asbp_fpc_fast_runner_farmer (Utilities|Casting|CastToBP_FPC_FastRunnerFarmer _returnvalue))
    (Variables|/Game/FarmerChar/BP_FPC_FastRunnerFarmer.BP_FPC_FastRunnerFarmer_C|SetPlantsGathered _asbp_fpc_fast_runner_farmer 0)
    (bind _needplants (CallFunction|CalculateNewPlantsCount (Variables|Default|GetNeedPlants)))
    (bind _output_get (Variables|Default|SetNeedPlants _needplants))
    (Variables|Default|SetHeaderText (Utilities|String|ToString(Text) (Utilities|Text|ToText(Integer) _output_get)))
    (return (>= (Variables|Default|GetCurrentPlants) (Variables|Default|GetNeedPlants)))))

(fn CalculateNewPlantsCount
  (params (NowPlants :type Integer))
  (return (+ NowPlants 2)))