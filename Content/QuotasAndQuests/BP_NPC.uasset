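; NPC actor that shows dialogue and can hand out quests through a WBP_Dialogue widget.
; Interact starts Talk only while IsActive, which this graph never sets true.
; Talk reuses or creates the widget, fills name, text and portrait from the Dialogue array, and passes any quest to its QuestHolder.
; It re-calls itself after a short delay until EndDialogue removes the widget and resets state.
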(event OnComponentEndOverlap(Sphere)
  (params (OverlappedComponent :type Primitive%20Component%20Object%20Reference) (OtherActor :type Actor%20Object%20Reference) (OtherComp :type Primitive%20Component%20Object%20Reference) (OtherBodyIndex :type Integer)))

(event EventBeginPlay
  (Variables|Default|SetIsActive false))

(event Collision|EventActorBeginOverlap
  (params (OtherActor :type Actor%20Object%20Reference)))

(event EventTick
  (params (DeltaSeconds :type Float%20%28single-precision%29)))

(event EventInteract
  (if (Variables|Default|GetIsActive)
    (Default|Talk self)))

(event EventTalk
  (bind _talkindex (Variables|Default|GettalkIndex))
  (bind _dialogue (Variables|Default|Getdialogue))
  (bind _output (Utilities|Array|Get(acopy) _dialogue _talkindex))
  (bind _myquest (Variables|/Game/QuotasAndQuests/BP_Dialogue.BP_Dialogue_C|GetMyQuest _output))
  (Math|Integer|IncrementInt (Variables|Default|GettalkIndex)
    (:%20%20
      (Development|PrintString "Hello")
      (if (< (Variables|Default|GettalkIndex) (Utilities|Array|Length (Variables|Default|Getdialogue)))
        (bind _uiwidget (Variables|Default|GetUIwidget)
          (:then
            (if (UserInterface|Viewport|IsinViewport _uiwidget)
              _
              (else
                (UserInterface|Viewport|AddtoViewport (stale _output_get) 0 :!label _label))))
          (:else
            (bind _returnvalue (UserInterface|CreateWidget "/Game/QuotasAndQuests/WBP_Dialogue.WBP_Dialogue_C" (Game|GetPlayerController 0)))
            (bind _output_get (Variables|Default|SetUIwidget _returnvalue))
            (goto _label)))
        (Utilities|FlowControl|Sequence
          (:then_0
            (Variables|/Script/UMG.TextBlock|SetText (Variables|/Game/QuotasAndQuests/WBP_Dialogue.WBP_Dialogue_C|GetNameText (Variables|Default|GetUIwidget)) (Utilities|Text|ToText(String) (Variables|/Game/QuotasAndQuests/BP_Dialogue.BP_Dialogue_C|GetName _output))))
          (:then_1
            (Variables|/Script/UMG.TextBlock|SetText (Variables|/Game/QuotasAndQuests/WBP_Dialogue.WBP_Dialogue_C|GetDialogueText (Variables|Default|GetUIwidget)) (Utilities|Text|ToText(String) (Variables|/Game/QuotasAndQuests/BP_Dialogue.BP_Dialogue_C|GetText _output))))
          (:then_2
            (Appearance|SetBrushfromTexture (Variables|/Game/QuotasAndQuests/WBP_Dialogue.WBP_Dialogue_C|GetPortrait (Variables|Default|GetUIwidget)) (Variables|/Game/QuotasAndQuests/BP_Dialogue.BP_Dialogue_C|GetPortrait _output) false))
          (:then_3
            (if (Variables|/Game/QuotasAndQuests/BP_Dialogue.BP_Dialogue_C|GetHasQuest _output)
              (Default|SetQuest (Variables|/Game/QuotasAndQuests/BP_Quest.BP_Quest_C|GetQuestHolder _myquest) _myquest)))
          (:then_4
            (Audio|PlaySound2D "/Engine/VREditor/Sounds/UI/Click_on_Button.Click_on_Button" 1.0 1.0 0.0 0 0)
            (Utilities|FlowControl|Delay 0.2)
            (Default|Talk self)))
        (else
          (Utilities|EndDialogue))))))

(fn ConstructionScript)