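; BP_CallDialogue plays a timed dialogue sequence on screen and can hand out quests along the way.
; Interact starts Talk only while IsActive is set, which happens outside this graph.
; Talk lazily creates WBP_Dialogue, fills name, text and portrait, passes any quest to its QuestHolder, then re-calls itself after SentenceDuration.
; After the last line it removes the widget, resets the index and deactivates.
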(event EventBeginPlay
  (Variables|Default|SetIsActive false))

(event EventInteract
  (if (Variables|Default|GetIsActive)
    (Default|Talk self)))

(event EventTalk
  (Math|Integer|IncrementInt (Variables|Default|GetTalk%20Index)
    (:%20%20
      (Development|PrintString "Hello")
      (if (< (Variables|Default|GetTalk%20Index) (Utilities|Array|Length (Variables|Default|Getdialogue)))
        (bind _uiwidget (Variables|Default|GetUIwidget)
          (:then
            (if (UserInterface|Viewport|IsinViewport _uiwidget)
              _
              (else
                (UserInterface|Viewport|AddtoViewport (stale _output_get) 0 :!label _label))))
          (:else
            (bind _returnvalue (UserInterface|CreateWidget "/Game/QuotasAndQuests/WBP_Dialogue.WBP_Dialogue_C" (Game|GetPlayerController 0)))
            (bind _output_get (Variables|Default|SetUIwidget _returnvalue))
            (goto _label)))
        (Utilities|FlowControl|Sequence
          (:then_0
            (Variables|/Script/UMG.TextBlock|SetText (Variables|/Game/QuotasAndQuests/WBP_Dialogue.WBP_Dialogue_C|GetNameText (Variables|Default|GetUIwidget)) (Utilities|Text|ToText(String) (Variables|/Game/QuotasAndQuests/BP_Dialogue.BP_Dialogue_C|GetName (Utilities|Array|Get(acopy) (Variables|Default|Getdialogue) (Variables|Default|GetTalk%20Index))))))
          (:then_1
            (Variables|/Script/UMG.TextBlock|SetText (Variables|/Game/QuotasAndQuests/WBP_Dialogue.WBP_Dialogue_C|GetDialogueText (Variables|Default|GetUIwidget)) (Utilities|Text|ToText(String) (Variables|/Game/QuotasAndQuests/BP_Dialogue.BP_Dialogue_C|GetText (Utilities|Array|Get(acopy) (Variables|Default|Getdialogue) (Variables|Default|GetTalk%20Index))))))
          (:then_2
            (Appearance|SetBrushfromTexture (Variables|/Game/QuotasAndQuests/WBP_Dialogue.WBP_Dialogue_C|GetPortrait (Variables|Default|GetUIwidget)) (Variables|/Game/QuotasAndQuests/BP_Dialogue.BP_Dialogue_C|GetPortrait (Utilities|Array|Get(acopy) (Variables|Default|Getdialogue) (Variables|Default|GetTalk%20Index))) false))
          (:then_3
            (if (Variables|/Game/QuotasAndQuests/BP_Dialogue.BP_Dialogue_C|GetHasQuest (Utilities|Array|Get(acopy) (Variables|Default|Getdialogue) (Variables|Default|GetTalk%20Index)))
              (Default|SetQuest (Variables|/Game/QuotasAndQuests/BP_Quest.BP_Quest_C|GetQuestHolder (Variables|/Game/QuotasAndQuests/BP_Dialogue.BP_Dialogue_C|GetMyQuest (Utilities|Array|Get(acopy) (Variables|Default|Getdialogue) (Variables|Default|GetTalk%20Index)))) (Variables|/Game/QuotasAndQuests/BP_Dialogue.BP_Dialogue_C|GetMyQuest (Utilities|Array|Get(acopy) (Variables|Default|Getdialogue) (Variables|Default|GetTalk%20Index))))))
          (:then_4
            (Audio|PlaySound2D "/Engine/VREditor/Sounds/UI/Click_on_Button.Click_on_Button" 1.0 1.0 0.0 0 0)
            (Utilities|FlowControl|Delay (Variables|Default|GetSentenceDuration))
            (Default|Talk self)))
        (else
          (bind _uiwidget_2 (Variables|Default|GetUIwidget)
            (:then
              (Widget|RemovefromParent _uiwidget_2)
              (Variables|Default|SetTalk%20Index -1)
              (Variables|Default|SetIsActive false))
            (:else)))))))

(fn ConstructionScript)