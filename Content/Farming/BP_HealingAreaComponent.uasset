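; BP_HealingAreaComponent is a farming component that makes a plant periodically heal actors around it.
; On BeginPlay it adds a translucent-style aura sphere mesh without collision and a sphere collider sized by the healing range to the Plant.
; A looping timer then polls the collider's overlapping actors and calls Heal on any with a BP_HealthComponent.
; The aura's scale is fixed, independent of the healing range.
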(event Custom|Proc%20Heal
  (for _array_element (Collision|GetOverlappingActors (Variables|Default|GetCollider) 0 :!class /Script/Engine.PrimitiveComponent)
    (if (Utilities|IsValid (Actor|GetComponentbyClass _array_element "/Game/FirstPerson/Blueprints/BP_HealthComponent.BP_HealthComponent_C"))
      (Default|Heal (Actor|GetComponentbyClass _array_element "/Game/FirstPerson/Blueprints/BP_HealthComponent.BP_HealthComponent_C") (Variables|Default|GetHeal%20Force)))))

(event EventBeginPlay
  (|CallParentFunction)
  (Utilities|FlowControl|Sequence
    (:then_0
      (bind _returnvalue (Game|AddComponentbyClass (Variables|Default|GetPlant) "/Script/Engine.StaticMeshComponent" false (Math|Transform|MakeTransform "0.000000,0.000000,100.000000")))
      (bind _output_get (Variables|Default|SetAura%20Sphere _returnvalue))
      (Components|StaticMesh|SetStaticMesh _output_get "/Engine/BasicShapes/Sphere.Sphere")
      (Rendering|Material|SetMaterial _output_get 0 "/Game/Farming/Materials/M_Aura_Inst.M_Aura_Inst")
      (Collision|SetCollisionEnabled (Variables|Default|GetAura%20Sphere) "NoCollision")
      (Transformation|SetRelativeScale3D (Variables|Default|GetAura%20Sphere) (* (Math|Vector|MakeVector 1.0 1.0 1.0) 5.0)))
    (:then_1
      (bind _returnvalue_2 (Game|AddComponentbyClass (Variables|Default|GetPlant) "/Script/Engine.SphereComponent" false))
      (bind _output_get_2 (Variables|Default|SetCollider _returnvalue_2))
      (Components|Sphere|SetSphereRadius _output_get_2 (Variables|Default|GetHealindg%20Range) true)
      (Rendering|SetVisibility _output_get_2 true false))
    (:then_2
      (Utilities|Time|SetTimerbyEvent (delegate Custom|Proc%20Heal) (Variables|Default|GetProc%20Rate) true true))))