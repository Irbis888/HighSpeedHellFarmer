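; BP_WaterPuddle is a temporary puddle actor that waters BP_Plant actors within its sphere and destroys itself after LifeTime.
; A one-second looping timer calls GetWater on each overlapping plant.
; The construction script sizes the collision sphere and Niagara sprite from Radius.
; Tick steadily lowers the sprite-to-radius ratio, so the visual shrinks while the watering radius is reapplied unchanged.
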(event Custom|Water%20Up
  (for _array_element (Collision|GetOverlappingActors (Variables|Default|GetSphere) "/Game/Farming/BP_Plant.BP_Plant_C" :!class /Script/Engine.PrimitiveComponent)
    (Default|GetWater (.AsBP%20Plant (Utilities|Casting|CastToBP_Plant _array_element)))))

(event Custom|Kill
  (Actor|DestroyActor))

(event EventBeginPlay
  (Utilities|Time|SetTimerbyEvent (delegate Custom|Water%20Up) 1.0 true)
  (Utilities|Time|SetTimerbyEvent (delegate Custom|Kill) (Variables|Default|GetLife%20Time)))

(event Collision|EventActorBeginOverlap
  (params (OtherActor :type Actor%20Object%20Reference)))

(event EventTick
  (params (DeltaSeconds :type Float%20%28single-precision%29))
  (Variables|Default|SetnsColliderRatio (- (Variables|Default|GetnsColliderRatio) (* DeltaSeconds 0.5)))
  (Components|Sphere|SetSphereRadius (Variables|Default|GetSphere) (Variables|Default|GetRadius) true)
  (Niagara|SetNiagaraVariable(Float) (Variables|Default|GetVFX) "Uniform Sprite Size" (* (Variables|Default|GetRadius) (Variables|Default|GetnsColliderRatio))))

(fn ConstructionScript
  (Components|Sphere|SetSphereRadius (Variables|Default|GetSphere) (Variables|Default|GetRadius) true)
  (Niagara|SetNiagaraVariable(Float) (Variables|Default|GetVFX) "Uniform Sprite Size" (* (Variables|Default|GetRadius) (Variables|Default|GetnsColliderRatio))))