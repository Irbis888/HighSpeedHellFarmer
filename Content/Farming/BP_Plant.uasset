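; Farmable plant actor configured by PlantStruct, which supplies its mesh, growth and drying speeds, drop and extra components loaded asynchronously.
; Each tick it dries out, destroys itself when moisture drops below zero, scales its body with growth, and updates a player-yaw-aligned moisture/growth widget.
; Overlapping BP_Water_P restores moisture.
; Interacting when collectable and nearly grown credits the player, spawns a homing item drop and destroys the plant.
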(event Custom|Get%20Water
  (Variables|Default|SetMoisture (Math|Float|Clamp(Float) (+ (Variables|Default|GetMoisture) 0.6))))

(event EventBeginPlay
  (Variables|Default|SetStartScale (Transformation|GetWorldScale (Variables|Default|GetBody)))
  (for _array_element (Utilities|Struct|BreakS_Plant (Variables|Default|GetPlantStruct))
    (Utilities|AsyncLoadClassAsset _array_element
      (:Completed
        (Game|AddComponentbyClass (Utilities|ResolveSoftReference _array_element))))))

(event EventTick
  (params (DeltaSeconds :type Float%20%28single-precision%29))
  (bind _moistbar (Variables|Default|GetMoistBar))
  (bind _returnvalue (Transformation|GetWorldRotation _moistbar))
  (Utilities|FlowControl|Sequence
    (:then_0
      (Transformation|SetWorldRotation _moistbar (Math|Rotator|MakeRotator (.roll _returnvalue) (.pitch _returnvalue) (+ (.yaw (Transformation|GetActorRotation (Game|GetPlayerCharacter 0))) 1.8e+02)) false false))
    (:then_1
      (bind _aswb_moisture_bar (Utilities|Casting|CastToWB_MoistureBar (UserInterface|GetWidget (Variables|Default|GetMoistBar))))
      (Progress|SetPercent (Variables|/Game/MapParts/WB_MoistureBar.WB_MoistureBar_C|GetMoistureBar _aswb_moisture_bar) (Variables|Default|GetMoisture))
      (Progress|SetPercent (Variables|/Game/MapParts/WB_MoistureBar.WB_MoistureBar_C|GetGrowthBar _aswb_moisture_bar) (Variables|Default|GetGrowth)))
    (:then_2
      (bind _output_get (Variables|Default|SetMoisture (- (Variables|Default|GetMoisture) (* (Variables|Default|GetDrySpeed) DeltaSeconds))))
      (if (< _output_get 0.0)
        (Actor|DestroyActor)))
    (:then_3
      (CallFunction|UpdGrowth DeltaSeconds))))

(event Collision|EventActorBeginOverlap
  (params (OtherActor :type Actor%20Object%20Reference))
  (Utilities|Casting|CastToBP_Water_P OtherActor)
  (CallFunction|GetWater))

(event EventInteract
  (if (and (Variables|Default|GetToCollect) (> (Variables|Default|GetGrowth) 0.96))
    (Default|AddPlants (.AsBP%20FPC%20Fast%20Runner%20Farmer (Utilities|Casting|CastToBP_FPC_FastRunnerFarmer (Game|GetPlayerCharacter 0))) 1)
    (Game|SpawnActorfromClass "/Game/Inventory/BP_ItemEntity.BP_ItemEntity_C" (Transformation|GetActorTransform) "Undefined" "MultiplyWithRoot" 0 (Utilities|Array|Get(acopy) (.Drop (Utilities|Struct|BreakS_Plant (Variables|Default|GetPlantStruct)))) true true 4e+01 0)
    (Actor|DestroyActor)))

(fn ConstructionScript
  (bind _plantstruct (Variables|Default|GetPlantStruct))
  (bind (_dryspeed _mesh) (Utilities|Struct|BreakS_Plant _plantstruct))
  (Variables|Default|SetGrowthSpeed (.GrowthSpeed (Utilities|Struct|BreakS_Plant (Variables|Default|GetPlantStruct))))
  (Variables|Default|SetDrySpeed _dryspeed)
  (Components|StaticMesh|SetStaticMesh (Variables|Default|GetBody) _mesh))

(fn UpdGrowth
  (params (Delta :type Float%20%28double-precision%29))
  (if (Utilities|IsValid (Variables|Default|GetBody))
    (Variables|Default|SetGrowth (Math|Float|Clamp(Float) (+ (Variables|Default|GetGrowth) (* (Variables|Default|GetGrowthSpeed) Delta))))
    (Transformation|SetWorldScale3D (Variables|Default|GetBody) (* (Variables|Default|GetStartScale) (Variables|Default|GetGrowth)))))