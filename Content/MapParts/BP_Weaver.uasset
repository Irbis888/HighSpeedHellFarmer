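; BP_Weaver is a timed emitter actor that repeatedly spawns seed actors of a configurable class at its own location until its lifetime runs out.
; BeginPlay starts a looping timer at FireRate that calls SpawnSeed, which spawns each actor with a random downward pitch, random yaw and the emitter's scale.
; Each spawn subtracts FireRate from Lifetime, and the emitter destroys itself once that drops below zero.
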(event Custom|SpawnSeed
  (bind _returnvalue (Transformation|GetActorTransform))
  (Game|SpawnActorfromClass (Variables|Default|GetSpawning%20Class) (Math|Transform|MakeTransform (.location _returnvalue) (Math|Rotator|MakeRotator 0.0 (Math|Random|RandomFloatinRange -25.0 -45.0) (Math|Random|RandomFloatinRange 0.0 3.6e+02)) (.scale _returnvalue)) "AlwaysSpawn" "MultiplyWithRoot" 0 0)
  (bind _output_get (Variables|Default|SetLifetime (- (Variables|Default|GetLifetime) (Variables|Default|GetFireRate))))
  (if (< _output_get 0.0)
    (Actor|DestroyActor)))

(event EventBeginPlay
  (Utilities|Time|SetTimerbyEvent (delegate Custom|SpawnSeed) (Variables|Default|GetFireRate) true))

(event Collision|EventActorBeginOverlap
  (params (OtherActor :type Actor%20Object%20Reference)))

(event EventTick
  (params (DeltaSeconds :type Float%20%28single-precision%29)))

(fn ConstructionScript)