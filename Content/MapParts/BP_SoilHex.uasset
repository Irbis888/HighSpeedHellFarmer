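; BP_SoilHex is a soil hex map part that hosts a single BP_Plant.
; Interacting with it spawns a plant at the PlantPoint transform, owned by the hex, and stores the reference if no valid plant exists.
; SummonPlant uses the same empty-slot check and spawn, but also passes plant struct data into the new plant.
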(event EventBeginPlay)

(event Collision|EventActorBeginOverlap
  (params (OtherActor :type Actor%20Object%20Reference)))

(event EventTick
  (params (DeltaSeconds :type Float%20%28single-precision%29)))

(event EventInteract
  (if (not (Utilities|IsValid (Variables|Default|GetPlant)))
    (bind _returnvalue (Game|SpawnActorfromClass :Class "/Game/Farming/BP_Plant.BP_Plant_C" :SpawnTransform (Transformation|GetWorldTransform (Variables|Default|GetPlantPoint)) :CollisionHandlingOverride "Undefined" :TransformScaleMethod "MultiplyWithRoot" :Owner self :Instigator 0))
    (Variables|Default|SetPlant _returnvalue)))

(fn ConstructionScript)

(fn SummonPlant
  (params (Plant :type S%20Plant%20Structure))
  (if (not (Utilities|IsValid (Variables|Default|GetPlant)))
    (bind _returnvalue (Game|SpawnActorfromClass "/Game/Farming/BP_Plant.BP_Plant_C" (Transformation|GetWorldTransform (Variables|Default|GetPlantPoint)) "Undefined" "MultiplyWithRoot" self Plant 0))
    (Variables|Default|SetPlant _returnvalue)))