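; Procedural map generator that builds a hex-style tile grid of soil, lava and rock in the construction script.
; Depending on Type, MakeMap fills the GenMap array with one hex type, or MakeLake puts a lowered lava patch in the centre of soil.
; CreateMap converts each index to staggered-row coordinates, adding child actors for soil and static mesh components for lava and rock.
; The EventGraph generation code is unconnected.
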(event EventBeginPlay)

(event Collision|EventActorBeginOverlap
  (params (OtherActor :type Actor%20Object%20Reference)))

(fn ConstructionScript
  (Utilities|Array|Resize (Variables|Default|GetGenMap) (* (Variables|Default|GetLength) (Variables|Default|GetWidth)))
  (switch Utilities|FlowControl|Switch|SwitchonMapType (Variables|Default|GetType)
    (:NewEnumerator0
      (CallFunction|MakeMap))
    (:NewEnumerator1
      (CallFunction|MakeLake)))
  (CallFunction|CreateMap))

(fn MakeMap
  (for _index (range 1 (Variables|Default|GetLength))
    (for _index_2 (range 1 (Variables|Default|GetWidth))
      (LocalVariables|Seti _index)
      (LocalVariables|Setj _index_2)
      (Utilities|Array|SetArrayElem (Variables|Default|GetGenMap) (+ (* (Variables|Default|GetWidth) (LocalVariables|Geti)) (LocalVariables|Getj)) (Utilities|Struct|MakeGenElement (Variables|Default|GetHexType) 0.0)))))

(fn CreateMap
  (bind _width (Variables|Default|GetWidth))
  (for (_array_element _array_index) (Variables|Default|GetGenMap)
    (switch Utilities|FlowControl|Switch|SwitchonHexType (.Type (Utilities|Struct|BreakGenElement _array_element))
      (:NewEnumerator1
        _)
      (:NewEnumerator2
        _)
      (:NewEnumerator3
        _))
    (LocalVariables|Seti (/ _array_index _width))
    (LocalVariables|Setj (Math|Integer|%(Integer) _array_index _width))
    (LocalVariables|SetAdjust (.AltAdjust (Utilities|Struct|BreakGenElement _array_element)))
    (if (== (Math|Integer|%(Integer) (LocalVariables|Getj) 2) 0)
      (Variables|Default|SetCoord (Math|Vector|MakeVector (* (LocalVariables|Geti) (Variables|Default|GetHorizDistance)) (* (LocalVariables|Getj) (Variables|Default|GetVertDistance)) (LocalVariables|GetAdjust)))
      (else
        (Variables|Default|SetCoord (Math|Vector|MakeVector (+ (* (LocalVariables|Geti) (Variables|Default|GetHorizDistance)) (/ (Variables|Default|GetHorizDistance) 2.0)) (* (LocalVariables|Getj) (Variables|Default|GetVertDistance)) (LocalVariables|GetAdjust)))))
    (LocalVariables|SetToSpawn (Math|Transform|MakeTransform (Variables|Default|GetCoord)))
    (switch Utilities|FlowControl|Switch|SwitchonHexType (.Type (Utilities|Struct|BreakGenElement _array_element))
      (:NewEnumerator1
        (AddComponent|AddChildActorComponent false (LocalVariables|GetToSpawn)))
      (:NewEnumerator2
        (AddComponent|AddStaticMeshComponent false (LocalVariables|GetToSpawn)))
      (:NewEnumerator3
        (AddComponent|AddStaticMeshComponent false (LocalVariables|GetToSpawn))))))

(fn MakeLake
  (for _index (range 1 (Variables|Default|GetLength))
    (for _index_2 (range 1 (Variables|Default|GetWidth))
      (LocalVariables|Seti _index)
      (LocalVariables|Setj _index_2)
      (if (and (< (Math|Integer|Absolute(Integer) (- (LocalVariables|Geti) (/ (Variables|Default|GetLength) 2))) 3) (< (Math|Integer|Absolute(Integer) (- (LocalVariables|Getj) (/ (Variables|Default|GetWidth) 2))) 3))
        (Utilities|Array|SetArrayElem (Variables|Default|GetGenMap) (+ (* (Variables|Default|GetWidth) (LocalVariables|Geti)) (LocalVariables|Getj)) (Utilities|Struct|MakeGenElement "NewEnumerator2" -5e+01))
        (else
          (Utilities|Array|SetArrayElem (Variables|Default|GetGenMap) (+ (* (Variables|Default|GetWidth) (LocalVariables|Geti)) (LocalVariables|Getj)) (Utilities|Struct|MakeGenElement "NewEnumerator1" 0.0)))))))