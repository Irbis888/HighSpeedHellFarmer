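; BP_Enemy is an enemy creature with a health bar widget and basic, test-like damage handling.
; On BeginPlay it copies its Health and MaxHealth into the WB_HealthBar widget held by its HealthBar component.
; Interact makes the enemy apply fixed damage to itself, credited to the first player controller.
; AnyDamage only prints the amount, leaving Health and the bar unchanged.
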(event EventBeginPlay
  (bind _output_get (Variables|Default|SetHBar%20Widget (.AsWB%20Health%20Bar (Utilities|Casting|CastToWB_HealthBar (UserInterface|GetWidget (Variables|Default|GetHealthBar))))))
  (Variables|/Game/UI/WB_HealthBar.WB_HealthBar_C|SetMaxHealth _output_get (Variables|Default|GetMaxHealth))
  (Variables|/Game/UI/WB_HealthBar.WB_HealthBar_C|SetHealth _output_get (Variables|Default|GetHealth)))

(event Game|Damage|EventAnyDamage
  (params (Damage :type Float%20%28single-precision%29) (DamageType :type Damage%20Type%20Object%20Reference) (InstigatedBy :type Controller%20Object%20Reference) (DamageCauser :type Actor%20Object%20Reference))
  (Development|PrintString (Utilities|String|ToString(Float) Damage)))

(event EventInteract
  (bind _returnvalue (Game|GetPlayerController 0))
  (Game|Damage|ApplyDamage self 15.0 _returnvalue _returnvalue))

(fn ConstructionScript)