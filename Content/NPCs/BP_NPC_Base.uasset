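; BP_NPC_Base is a base NPC that a manager can move in scripted scenarios and that shows dialogue when interacted with.
; ScenarioMove sends it to MoveTarget via AI MoveTo, then flags Manager.Ready whether the move succeeds or fails.
; Interact calls Say with a hardcoded Russian line, creating a WBP_Dialogue widget with the portrait and name from Info.
; GoToActor is an empty stub, and a debug move to the player is left unconnected.
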(event Custom|Scenario%20Move
  (AI|AIMoveTo self "-1000.000000,-1000.000000,0.000000" (Variables|Default|GetMove%20Target) 5.0 true
    (:OnSuccess
      _)
    (:OnFail
      _))
  (CallFunction|NotifyManager))

(event Custom|Notify%20Manager
  (Variables|/Game/NPCs/EventSystem/BP_EventManager.BP_EventManager_C|SetReady (Variables|Default|GetManager) true))

(event EventBeginPlay)

(event EventInteract
  (CallFunction|Say "Я ведомая кукла" 0.0))

(fn ConstructionScript)

(fn Say
  (params (Text :type Text) (Duration :type Float%20%28single-precision%29))
  (bind _info (Variables|Default|GetInfo))
  (bind (_portrait _displayname) (Utilities|Struct|BreakS_NPCInfo _info))
  (bind _returnvalue (UserInterface|CreateWidget "/Game/QuotasAndQuests/WBP_Dialogue.WBP_Dialogue_C" (Game|GetPlayerController 0) Text _portrait _displayname Duration))
  (UserInterface|Viewport|AddtoViewport _returnvalue 0))

(fn GotoActor)