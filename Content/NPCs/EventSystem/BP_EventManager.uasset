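; BP_EventManager is a scenario sequencer that plays an ordered list of scripted NPC commands, starting on the tick after BeginPlay.
; Proceed runs the current entry: move an assigned actor, delay, activate a BP_Trigger, or make an actor speak.
; Delay and Say raise a Ready flag when finished, which Tick polls to advance.
; Move and Wait Trigger leave Ready untouched here, so advancing past them requires an external signal.
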(event Custom|Start%20Execution
  (Variables|Default|SetCurrentEvent 0)
  (Class|KismetSystemLibrary|SetTimerforNextTickDelegate (delegate Custom|Proceed)))

(event Custom|Proceed
  (bind _scenariolist (Variables|Default|GetScenarioList))
  (bind _currentevent (Variables|Default|GetCurrentEvent))
  (bind _output (Utilities|Array|Get(acopy) _scenariolist _currentevent))
  (bind (_command _floatarg _intarg _assignedactor _actortarget _textarg) (Utilities|Struct|BreakS_ScenarioEvent _output))
  (Development|PrintString (Utilities|String|EnumtoString _command))
  (switch Utilities|FlowControl|Switch|SwitchonE_Commands _command
    (:NewEnumerator0
      (Variables|/Game/NPCs/BP_NPC_Base.BP_NPC_Base_C|SetMove%20Target _assignedactor _actortarget)
      (Default|ScenarioMove _assignedactor))
    (:NewEnumerator1
      (Utilities|FlowControl|Delay _floatarg)
      (Variables|Default|SetReady true :!label _label))
    (:NewEnumerator2
      (Variables|/Game/NPCs/EventSystem/BP_Trigger.BP_Trigger_C|SetActive (.AsBP%20Trigger (Utilities|Casting|CastToBP_Trigger _actortarget)) true))
    (:NewEnumerator3
      (Default|Say _assignedactor _textarg _floatarg)
      (Utilities|FlowControl|Delay _floatarg)
      (goto _label))))

(event Custom|Next
  (bind _result (Math|Integer|IncrementInt (Variables|Default|GetCurrentEvent))
    (:%20%20
      (Variables|Default|SetReady false)
      (if (not (>= _result (Utilities|Array|Length (Variables|Default|GetScenarioList))))
        (CallFunction|Proceed)))))

(event EventBeginPlay
  (CallFunction|StartExecution))

(event EventTick
  (params (DeltaSeconds :type Float%20%28single-precision%29))
  (if (Variables|Default|GetReady)
    (CallFunction|Next)))

(fn ConstructionScript)

(fn Sendto
  (params (Target%20Actor :type Actor%20Object%20Reference) (Walking%20Actor :type BP%20NPC%20Base%20Object%20Reference))
  (AI|Navigation|MovetoActor (AI|GetAIController Walking%20Actor) Target%20Actor 5.0 true true true 0))