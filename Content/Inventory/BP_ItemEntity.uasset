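; BP_ItemEntity is a physics-simulated dropped item in the world, showing the mesh of its Item data.
; It becomes pickupable after a short timer from BeginPlay, then a sphere overlap by the farmer character adds the Item to that character's inventory component and destroys the actor.
; When Attracting is set, it disables gravity and homes toward the player through velocity-change impulses every tick.
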(event OnComponentBeginOverlap(Sphere)
  (params (OverlappedComponent :type Primitive%20Component%20Object%20Reference) (OtherActor :type Actor%20Object%20Reference) (OtherComp :type Primitive%20Component%20Object%20Reference) (OtherBodyIndex :type Integer) (bFromSweep :type Boolean) (SweepResult :type Hit%20Result%20Structure%20%28by%20ref%29))
  (if (Variables|Default|GetPickupable)
    (bind _asbp_fpc_fast_runner_farmer (Utilities|Casting|CastToBP_FPC_FastRunnerFarmer OtherActor))
    (Default|AddItem (Variables|/Game/FarmerChar/BP_FPC_FastRunnerFarmer.BP_FPC_FastRunnerFarmer_C|GetBP_InventoryComp _asbp_fpc_fast_runner_farmer) (Variables|Default|GetItem))
    (Actor|DestroyActor)))

(event Custom|Make%20Pickupable
  (Variables|Default|SetPickupable true)
  (Utilities|Time|ClearandInvalidateTimerbyHandle (stale EventBeginPlay _returnvalue)))

(event EventBeginPlay
  (bind _returnvalue (Utilities|Time|SetTimerbyEvent (delegate Custom|Make%20Pickupable) 3.0))
  (if (Variables|Default|GetAttracting)
    (Physics|SetEnableGravity (Variables|Default|GetBody) false)))

(event Collision|EventActorBeginOverlap
  (params (OtherActor :type Actor%20Object%20Reference)))

(event EventTick
  (params (DeltaSeconds :type Float%20%28single-precision%29))
  (if (Variables|Default|GetAttracting)
    (Physics|AddImpulse (Variables|Default|GetBody) (* (Math|Vector|Normalize (- (Transformation|GetActorLocation (Game|GetPlayerCharacter 0)) (Transformation|GetActorLocation))) (Variables|Default|GetHomingForce)) "None" true)))

(fn ConstructionScript
  (Components|StaticMesh|SetStaticMesh (Variables|Default|GetBody) (.mesh (Variables|Default|GetItem)))
  (Physics|SetSimulatePhysics (Variables|Default|GetBody) true))